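; Camera volume actor that notifies overlapping actors implementing BPI_PlayerCamera when they enter or exit, passing itself in the message.
; Overlaps also call enter and exit functions for any actor and for players, all left empty here.
; While active and set to follow, Tick smoothly rotates VolumeCamera toward player character 0 using RInterpTo.
; Two custom events toggle the active state.
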(event Custom|CustomEvent_1
  (params (Player :type Actor%20Object%20Reference))
  (Variables|Default|SetIsActive? true))

(event Custom|CustomEvent
  (params (Player :type Actor%20Object%20Reference))
  (Variables|Default|SetIsActive? false))

(event Collision|EventActorBeginOverlap
  (params (OtherActor :type Actor%20Object%20Reference))
  (CallFunction|OnActorEnter OtherActor)
  (if (Utilities|DoesObjectImplementInterface OtherActor "/Game/BP/BPI_PlayerCamera.BPI_PlayerCamera_C")
    (CallFunction|OnPlayerEnter OtherActor)
    (Class|BPIPlayerCamera|VolumeEntered(Message) OtherActor self)))

(event EventTick
  (params (DeltaSeconds :type Float%20%28single-precision%29))
  (if (and (Variables|Default|GetIsActive?) (Variables|Default|GetMustFollowPlayer?))
    (Transformation|SetWorldRotation (Variables|Default|GetVolumeCamera) (CallFunction|InterpLooktoPlayer DeltaSeconds (Variables|Default|GetFollowInterpSpeed)) false false)))

(event Collision|EventActorEndOverlap
  (params (OtherActor :type Actor%20Object%20Reference))
  (CallFunction|OnActorExit OtherActor)
  (if (Utilities|DoesObjectImplementInterface OtherActor "/Game/BP/BPI_PlayerCamera.BPI_PlayerCamera_C")
    (CallFunction|OnPlayerExit OtherActor)
    (Class|BPIPlayerCamera|VolumeExited(Message) OtherActor self)))

(fn ConstructionScript
  (Variables|Default|SetVolumeTransform ""))

(fn OnActorEnter
  (params (Actor :type Actor%20Object%20Reference)))

(fn OnPlayerEnter
  (params (Player :type Actor%20Object%20Reference)))

(fn OnActorExit
  (params (Actor :type Actor%20Object%20Reference)))

(fn OnPlayerExit
  (params (Player :type Actor%20Object%20Reference)))

(fn InterpLooktoPlayer
  (params (DeltaSeconds :type Float%20%28single-precision%29) (InterpSpeed :type Float%20%28single-precision%29))
  (return (Math|Interpolation|RInterpTo (Transformation|GetWorldRotation (Variables|Default|GetVolumeCamera)) (Math|Rotator|FindLookatRotation (Transformation|GetWorldLocation (Variables|Default|GetVolumeCamera)) (Transformation|GetActorLocation (Game|GetPlayerCharacter 0))) DeltaSeconds InterpSpeed)))